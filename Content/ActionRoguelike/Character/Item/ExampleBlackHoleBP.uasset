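; Example black hole projectile actor that pulls in its surroundings and destroys what it touches, then removes itself after five seconds.
; Every tick a radial force component fires an impulse.
; Any actor overlapping its sphere component is destroyed, except the instigator, which the sphere also ignores when moving.
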(event OnComponentBeginOverlap(SphereComp)
  (params (OverlappedComponent :type Primitive%20Component%20Object%20Reference) (OtherActor :type Actor%20Object%20Reference) (OtherComp :type Primitive%20Component%20Object%20Reference) (OtherBodyIndex :type Integer) (bFromSweep :type Boolean) (SweepResult :type Hit%20Result%20Structure%20%28by%20ref%29))
  (if (not (== OtherActor (Variables|Default|GetInstigator)))
    (Actor|DestroyActor OtherActor)))

(event Custom|DestroySelf
  (Actor|DestroyActor))

(event EventBeginPlay
  (Utilities|Time|SetTimerbyEvent (delegate Custom|DestroySelf) 5.0)
  (Collision|IgnoreActorwhenMoving (Variables|Default|GetSphereComp) (Variables|Default|GetInstigator) true))

(event Collision|EventActorBeginOverlap
  (params (OtherActor :type Actor%20Object%20Reference)))

(event EventTick
  (params (DeltaSeconds :type Float%20%28single-precision%29))
  (Class|RadialForceComponent|FireImpulse (Variables|Default|GetRadialForce)))

(fn ConstructionScript)